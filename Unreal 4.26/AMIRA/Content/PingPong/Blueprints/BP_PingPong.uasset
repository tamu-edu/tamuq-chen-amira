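; BP_PingPong is an AR ping-pong actor with functions to persist its placement; its event graph is inactive.
; SaveGame pins the root component, stores that AR pin locally under AnchorName, then unpins it, leaving its transform-to-slot save disconnected.
; LoadGame does not read that pin: it restores the transform from BP_savegame, or creates the save with the current transform if none exists.
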(event EventBeginPlay)

(event Collision|EventActorBeginOverlap
  (params (OtherActor :type Actor%20Object%20Reference)))

(event EventTick
  (params (DeltaSeconds :type Float%20%28single-precision%29)))

(fn ConstructionScript)

(fn SaveGame
  (bind _defaultsceneroot (Variables|Default|GetDefaultSceneRoot))
  (bind _returnvalue (Class|ARBlueprintLibrary|PinComponent _defaultsceneroot (Transformation|GetWorldTransform _defaultsceneroot) 0))
  (bind _output_get (Variables|Default|SetPinned%20Component _returnvalue))
  (Class|ARBlueprintLibrary|SaveARPintoLocalStore (Variables|Default|GetAnchor%20Name) _output_get)
  (Class|ARBlueprintLibrary|UnpinComponent _defaultsceneroot))

(fn LoadGame
  (bind _returnvalue (SaveGame|DoesSaveGameExist "amira_1"))
  (if _returnvalue
    (bind _returnvalue_2 (SaveGame|LoadGamefromSlot "amira_1"))
    (bind _asbp_savegame (Utilities|Casting|CastToBP_savegame _returnvalue_2))
    (Transformation|SetActorTransform (Variables|/Game/PingPong/BP_savegame.BP_savegame_C|Getpingpong_pos _asbp_savegame))
    (else
      (bind _returnvalue_3 (SaveGame|CreateSaveGameObject "/Game/PingPong/BP_savegame.BP_savegame_C"))
      (Variables|/Game/PingPong/BP_savegame.BP_savegame_C|Setpingpong_pos _returnvalue_3 (Transformation|GetActorTransform))
      (SaveGame|SaveGametoSlot _returnvalue_3 "amira_1"))))