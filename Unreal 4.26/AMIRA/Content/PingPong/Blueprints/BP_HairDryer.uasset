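; Hair dryer actor in the PingPong game that blows physics objects along its up axis.
; While switched on, each tick fires a debug-drawn grid of line traces across its range, pushing simulating hits at the impact point by surface facing.
; UXT child-actor switch and slider control on/off and maximum force.
; Placement saves as a local AR pin and reloads from the pawn's loaded pins; save-slot code is unused.
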(event Custom|hairdryer_settings
  (bind _asuxt_pressable_switch_button_actor (Utilities|Casting|CastToUxtPressableSwitchButtonActor (Variables|/Script/Engine.ChildActorComponent|GetChildActor (Variables|Default|GetHairdryer_switch))))
  (EventDispatchers|BindEventtoOnToggled (Variables|/Script/UXTools.UxtPressableToggleButtonActor|GetToggleStateComponent _asuxt_pressable_switch_button_actor) (delegate Custom|switch))
  (bind _asuxt_pinch_slider_actor (Utilities|Casting|CastToUxtPinchSliderActor (Variables|/Script/Engine.ChildActorComponent|GetChildActor (Variables|Default|Gethairdryer_power))))
  (EventDispatchers|BindEventtoOnUpdateValue (Variables|/Script/UXTools.UxtPinchSliderActor|GetPinchSlider _asuxt_pinch_slider_actor) (delegate Custom|power_adjust)))

(event Custom|switch
  (params (ToggleState :type Uxt%20Toggle%20State%20Component%20Object%20Reference))
  (Variables|Default|SetHairBlowerOn? (Variables|/Script/UXTools.UxtToggleStateComponent|GetbIsChecked ToggleState)))

(event Custom|power_adjust
  (params (Slider :type Uxt%20Pinch%20Slider%20Component%20Object%20Reference) (NewValue :type Float%20%28single-precision%29))
  (bind _output_get (Variables|/Script/UXTools.UxtPinchSliderComponent|SetValue Slider NewValue))
  (Variables|Default|SetMax%20Force (* _output_get 1e+04)))

(event EventBeginPlay
  (CallFunction|HairdryerSettings))

(event EventTick
  (params (DeltaSeconds :type Float%20%28single-precision%29))
  (bind _returnvalue (Transformation|GetActorTransform))
  (bind _returnvalue_2 (Transformation|GetActorUpVector))
  (bind _distancebetweenforcelines (Variables|Default|GetDistanceBetweenForceLines))
  (if (Variables|Default|GetHairBlowerOn?)
    (for _index (range 0 (Math|Float|Truncate (/ (Variables|Default|GetRange%20X) (Variables|Default|GetDistanceBetweenForceLines))))
      (for _index_2 (range 0 (Math|Float|Truncate (/ (Variables|Default|GetRange%20Y) (Variables|Default|GetDistanceBetweenForceLines))))
        (bind (_outhit _returnvalue_3) (Collision|LineTraceByChannel (Math|Transform|TransformLocation _returnvalue (Math|Vector|MakeVector (- (* _index_2 _distancebetweenforcelines) (/ (Variables|Default|GetRange%20X) 2.0)) (- (* _index _distancebetweenforcelines) (/ (Variables|Default|GetRange%20Y) 2.0)) 0.0)) (Math|Transform|TransformLocation _returnvalue (+ (Math|Vector|MakeVector (- (* _index_2 _distancebetweenforcelines) (/ (Variables|Default|GetRange%20X) 2.0)) (- (* _index _distancebetweenforcelines) (/ (Variables|Default|GetRange%20Y) 2.0)) 0.0) (Math|Vector|MakeVector 0.0 0.0 (Variables|Default|GetRange%20Z)))) "TraceTypeQuery1" false 0 "ForOneFrame"))
        (if _returnvalue_3
          (if (Physics|IsSimulatingPhysics (.HitComponent (Collision|BreakHitResult _outhit)) "None")
            (Class|PrimitiveComponent|AddForceatLocation (.HitComponent (Collision|BreakHitResult _outhit)) (* (Math|Vector|Normalize (+ _returnvalue_2 (Math|Vector|NegateVector (.ImpactNormal (Collision|BreakHitResult _outhit))))) (* (Math|Float|Absolute(Float) (Math|Vector|DotProduct _returnvalue_2 (Math|Vector|NegateVector (.ImpactNormal (Collision|BreakHitResult _outhit))))) (Variables|Default|GetMax%20Force))) (.ImpactPoint (Collision|BreakHitResult _outhit)) "None")))))))

(fn ConstructionScript
  (bind _range (Variables|Default|GetRange))
  (Components|Box|SetBoxExtent _range (Math|Vector|MakeVector (/ (Variables|Default|GetRange%20X) 2.0) (/ (Variables|Default|GetRange%20Y) 2.0) (/ (Variables|Default|GetRange%20Z) 2.0)) true)
  (Transformation|SetRelativeLocation _range (Math|Vector|MakeVector 0.0 0.0 2e+02) false false))

(fn SaveGame
  (bind _defaultsceneroot (Variables|Default|GetDefaultSceneRoot))
  (bind _returnvalue (Class|ARBlueprintLibrary|PinComponent _defaultsceneroot (Transformation|GetWorldTransform _defaultsceneroot) 0))
  (bind _output_get (Variables|Default|SetpinnedComponent _returnvalue))
  (Class|ARBlueprintLibrary|SaveARPintoLocalStore (Variables|Default|GetAnchorName) _output_get)
  (Class|ARBlueprintLibrary|UnpinComponent _defaultsceneroot))

(fn LoadGame
  (bind _asbp_pawn (Utilities|Casting|CastToBP_Pawn (Game|Player|GetPlayerPawn 0)))
  (bind _values (Utilities|Map|Values (Variables|/Game/PingPong/Blueprints/BP_Pawn.BP_Pawn_C|GetLoaded%20ARPins _asbp_pawn)))
  (for _array_element _values
    (Development|PrintString (Utilities|String|ToString(Name) (Class|ARPin|GetDebugName _array_element)))
    (if (Utilities|Name|Equal(Name) (Class|ARPin|GetDebugName _array_element) (Variables|Default|GetAnchorName))
      (Utilities|IsValid (Class|ARPin|GetPinnedComponent _array_element)
        (:Is%20Valid
          (Transformation|AttachComponentToComponent (Class|ARPin|GetPinnedComponent _array_element) "None" "SnapToTarget" "SnapToTarget" "KeepWorld" true))
        (:Is%20Not%20Valid
          (Class|ARBlueprintLibrary|PinComponenttoARPin (Class|ARPin|GetPinnedComponent _array_element) _array_element)))
      (Development|PrintString "load"))))