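; BP_Menu is a UX Tools palm-up hand menu for spawning meshes and saving or loading anchors in mixed reality.
; On BeginPlay it hides the Admin component, binds three pressable buttons and caches Pingpong and Hairdryer references from BP_Pawn.
; Button handlers delegate to BP_Pawn, while the palm-up constraint toggles menu visibility.
; SaveGame and LoadGame helpers forward to both objects but are not wired to any event here.
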(event OnConstraintActivated(UxtPalmUpConstraint)
  (Class|UxtUIElementComponent|SetUIVisibility (Variables|Default|GetUxtUIElement) "Show"))

(event OnConstraintDeactivated(UxtPalmUpConstraint)
  (Class|UxtUIElementComponent|SetUIVisibility (Variables|Default|GetUxtUIElement) "Hide"))

(event Custom|Prepare%20Tabs
  (Rendering|SetVisibility (Variables|Default|GetAdmin) false true)
  (bind _asuxt_pressable_button_actor (Utilities|Casting|CastToUxtPressableButtonActor (Variables|/Script/Engine.ChildActorComponent|GetChildActor (Variables|Default|GetSpawn%20Mesh))))
  (EventDispatchers|BindEventtoOnButtonPressed (Variables|/Script/UXTools.UxtBasePressableButtonActor|GetButtonComponent _asuxt_pressable_button_actor) (delegate Custom|Spawn%20Meshes))
  (bind _asuxt_pressable_button_actor_2 (Utilities|Casting|CastToUxtPressableButtonActor (Variables|/Script/Engine.ChildActorComponent|GetChildActor (Variables|Default|GetSave_Button))))
  (EventDispatchers|BindEventtoOnButtonPressed (Variables|/Script/UXTools.UxtBasePressableButtonActor|GetButtonComponent _asuxt_pressable_button_actor_2) (delegate Custom|Save%20Anchor))
  (bind _asuxt_pressable_button_actor_3 (Utilities|Casting|CastToUxtPressableButtonActor (Variables|/Script/Engine.ChildActorComponent|GetChildActor (Variables|Default|GetLoad%20Anchor))))
  (EventDispatchers|BindEventtoOnButtonPressed (Variables|/Script/UXTools.UxtBasePressableButtonActor|GetButtonComponent _asuxt_pressable_button_actor_3) (delegate Custom|Load%20actor%20positions)))

(event Custom|Save%20Anchor
  (params (Button :type Uxt%20Pressable%20Button%20Component%20Object%20Reference) (Pointer :type Uxt%20Pointer%20Component%20Object%20Reference))
  (bind _asbp_pawn (Utilities|Casting|CastToBP_Pawn (Game|Player|GetPlayerPawn 0)))
  (Default|SaveLocalAnchor _asbp_pawn 0 "None"))

(event Custom|Prepare%20Spawn%20Tab)

(event Custom|Prepare%20Spatial%20Mapping%20Tab)

(event Custom|Prepare%20Anchor%20Tab)

(event Custom|Spawn%20Meshes
  (params (Button :type Uxt%20Pressable%20Button%20Component%20Object%20Reference) (Pointer :type Uxt%20Pointer%20Component%20Object%20Reference))
  (bind _asbp_pawn (Utilities|Casting|CastToBP_Pawn (Game|Player|GetPlayerPawn 0)))
  (Default|SpawnMesh _asbp_pawn))

(event Custom|Load%20actor%20positions
  (params (Button :type Uxt%20Pressable%20Button%20Component%20Object%20Reference) (Pointer :type Uxt%20Pointer%20Component%20Object%20Reference))
  (bind _asbp_pawn (Utilities|Casting|CastToBP_Pawn (Game|Player|GetPlayerPawn 0)))
  (Default|LoadPinsforObjects _asbp_pawn))

(event EventBeginPlay
  ;[1 1 1] Prepare all tabs and buttons
  (CallFunction|PrepareTabs)
  (bind _asbp_pawn (Utilities|Casting|CastToBP_Pawn (Game|Player|GetPlayerPawn 0)))
  (Variables|Default|Setpingpong (Variables|/Game/PingPong/Blueprints/BP_Pawn.BP_Pawn_C|GetPingpong _asbp_pawn))
  (Variables|Default|Sethairdryer (Variables|/Game/PingPong/Blueprints/BP_Pawn.BP_Pawn_C|GetHairdryer _asbp_pawn)))

(fn ConstructionScript)

(fn SaveGame
  (params (hairdryer :type BP%20Hair%20Dryer%20Object%20Reference) (pingpong :type BP%20Ping%20Pong%20Object%20Reference))
  (bind _returnvalue (SaveGame|DoesSaveGameExist "amira_1"))
  (if _returnvalue
    _
    (else
      (SaveGame|CreateSaveGameObject "/Game/PingPong/BP_savegame.BP_savegame_C")))
  (Default|SaveGame hairdryer)
  (Default|SaveGame pingpong))

(fn LoadGame
  (params (hairdryer :type BP%20Hair%20Dryer%20Object%20Reference) (pingpong :type BP%20Ping%20Pong%20Object%20Reference))
  (Default|LoadGame hairdryer)
  (Default|LoadGame pingpong))