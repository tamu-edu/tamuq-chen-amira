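; Mixed-reality player pawn that runs the AR session, renders tracked hands and manages ping-pong and hair dryer props.
; BeginPlay starts AR and spawns UXT hand interaction actors, then Tick copies hand keypoints onto hand mesh bones, mirroring left-hand Y scale.
; Separate events spawn the props, save or load them, attach components to named AR pins and collect tracked geometry.
; Head and eye-gaze debug traces are defined but not called here.
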(event OnUpdateTrackedGeometry(ARTrackableNotify)
  (params (TrackedGeometry :type AR%20Tracked%20Geometry%20Object%20Reference))
  (bind _returnvalue (Class|ARTrackedGeometry|GetUnderlyingMesh TrackedGeometry))
  ;[1 1 1] Collects Geometry Data
  (Utilities|IsValid _returnvalue
    (:Is%20Valid
      (if (Utilities|Enum|Equal(Enum) (.status (Class|ARBlueprintLibrary|GetARSessionStatus)) "Running")
        (Utilities|Array|AddUnique (Variables|Default|GetTracked%20Geometry) _returnvalue)))))

(event Custom|PrepareForAR
  ;[1 1 1] Prepare for AR
  (Class|ARBlueprintLibrary|StartARSession "/Game/PingPong/AR_SessionConfig.AR_SessionConfig")
  (CallFunction|SpawnHandInteraction))

(event Custom|EyeGrazeTracking
  (bind _hmdworldlocation (Variables|Default|GetHMDWorldLocation))
  ;[1 1 1] Track eyes
  (if (Class|EyeTrackerFunctionLibrary|IsEyeTrackerConnected)
    (bind (_outgazedata _returnvalue) (Class|EyeTrackerFunctionLibrary|GetGazeData))
    (if _returnvalue
      (Collision|LineTraceByChannel _hmdworldlocation (+ (* (.gazedirection _outgazedata) 5e+02) _hmdworldlocation) "TraceTypeQuery1" false 0 "ForOneFrame"))))

(event Custom|SpawnMesh
  ;[1 1 1] Spawn Meshes
  (bind _returnvalue (Game|SpawnActorfromClass "/Game/PingPong/Blueprints/BP_PingPong.BP_PingPong_C" (Math|Transform|MakeTransform "100.000000,-10.000000,130.000000" "0, 0, 0" "1,1,1") "AlwaysSpawn" 0 "pingpong" 0))
  (Variables|Default|SetPingpong _returnvalue)
  (bind _returnvalue_2 (Game|SpawnActorfromClass "/Game/PingPong/Blueprints/BP_HairDryer.BP_HairDryer_C" (Math|Transform|MakeTransform "100.000000,30.000000,80.000000" "0, 0,-90.000000" "1,1,1") "AlwaysSpawn" 0 "hairdryer" 0))
  (Variables|Default|SetHairdryer _returnvalue_2))

(event Custom|DeleteAllAnchors
  ;[1 1 1] Anchor Setup
  ;;[1 1 1] Delete All AR Anchors
  (Class|ARBlueprintLibrary|RemoveAllARPinsfromLocalStore)
  (Utilities|Map|Clear (Variables|Default|GetLoaded%20ARPins)))

(event Custom|SaveLocalAnchor
  (params (ComponentToPin :type Scene%20Component%20Object%20Reference) (DebugName :type Name))
  ;[1 1 1] Anchor Setup
  ;;[1 1 1] Save AR Anchors
  (Utilities|FlowControl|Sequence
    (:then_0
      (Default|SaveGame (Variables|Default|GetPingpong)))
    (:then_1
      (Default|SaveGame (Variables|Default|GetHairdryer)))))

(event Custom|HeadOrientationTracking
  ;[1 1 1] Track Head
  (bind _hmddata (Class|HeadMountedDisplayFunctionLibrary|GetHMDData self))
  (if (.bvalid _hmddata)
    (bind _output_get (Variables|Default|SetHMDWorldLocation (.position _hmddata)))
    (Collision|LineTraceByChannel _output_get (+ _output_get (* (Math|Vector|GetForwardVector (Class|KismetMathLibrary|QuatRotator (.rotation _hmddata))) 5e+02)) "TraceTypeQuery1" false 0 "ForOneFrame")))

(event Custom|AttachActorToPin
  (params (ComponentToPin :type Scene%20Component%20Object%20Reference) (DebugName :type Name))
  ;[1 1 1] Anchor Setup
  ;;[1 1 1] Setting Location of Object to AR Pin
  (bind _values (Utilities|Map|Values (Variables|Default|GetLoaded%20ARPins)))
  (for _array_element _values
    (if (Utilities|Name|Equal(Name) (Class|ARPin|GetDebugName _array_element) DebugName)
      (Utilities|IsValid (Class|ARPin|GetPinnedComponent _array_element)
        (:Is%20Valid
          (Transformation|AttachComponentToComponent (Components|GetOwner ComponentToPin) (Class|ARPin|GetPinnedComponent _array_element) "None" "SnapToTarget" "SnapToTarget" "KeepRelative" true))
        (:Is%20Not%20Valid
          (Class|ARBlueprintLibrary|PinComponenttoARPin ComponentToPin _array_element))))))

(event Custom|Load%20Pins%20for%20Objects
  ;[1 1 1] Anchor Setup
  ;;[1 1 1] Load AR Pins
  (Utilities|Map|Clear (Variables|Default|GetLoaded%20ARPins))
  (bind _returnvalue (Class|ARBlueprintLibrary|LoadARPinsfromLocalStore))
  (Variables|Default|SetLoaded%20ARPins _returnvalue)
  (Default|LoadGame (Variables|Default|GetHairdryer)))

(event Custom|SpawnHandInteraction
  (bind _returnvalue (Math|Transform|MakeTransform "0, 0, 0"))
  (bind _self self)
  ;[1 1 1] Hand Interaction UI
  (bind _returnvalue_2 (Game|SpawnActorfromClass "/Script/UXTools.UxtHandInteractionActor" _returnvalue "Undefined" _self true "Left" 0))
  (bind _returnvalue_3 (Game|SpawnActorfromClass "/Script/UXTools.UxtHandInteractionActor" _returnvalue "Undefined" _self true "Right" 0))
  (Utilities|IsValid (Actor|GetComponentbyClass _returnvalue_2 "/Script/UXTools.UxtFarCursorComponent")
    (:Is%20Valid
      (Variables|Default|SetLeftHandCursor (Actor|GetComponentbyClass _returnvalue_2 "/Script/UXTools.UxtFarCursorComponent"))
      (Variables|Default|SetRightHandCursor (Actor|GetComponentbyClass _returnvalue_3 "/Script/UXTools.UxtFarCursorComponent")))))

(event Custom|TrackHands
  (bind _left_hand (Variables|Default|GetLeft%20Hand))
  ;[1 1 1] Hand Tracking
  (for _index (range 0 1)
    (bind _motioncontrollerdata (Class|HeadMountedDisplayFunctionLibrary|GetMotionControllerData 0 (Utilities|Select :Index _index :Option%200 "Left" :Option%201 "Right")))
    (if (and (.bValid (Utilities|Struct|BreakXRMotionControllerData _motioncontrollerdata)) (Utilities|Enum|Equal(Enum) (.DeviceVisualType (Utilities|Struct|BreakXRMotionControllerData _motioncontrollerdata)) "Hand"))
      (bind _enumvalue (|ForEachEHandKeypoint)
        (:LoopBody
          (if (Transformation|DoesSocketExist (Variables|Default|GetRight%20Hand) (Utilities|RemoveSpaces _enumvalue))
            (switch Utilities|FlowControl|Switch|SwitchonEControllerHand (.HandIndex (Utilities|Struct|BreakXRMotionControllerData _motioncontrollerdata))
              (:Left
                (bind _adjustdata (CallFunction|ConvertTransform (Math|Transform|MakeTransform (Utilities|Array|Get(acopy) (.HandKeyPositions (Utilities|Struct|BreakXRMotionControllerData _motioncontrollerdata)) (Math|Conversions|ToInteger(Byte) _enumvalue)) (Class|KismetMathLibrary|QuatRotator (Utilities|Array|Get(acopy) (.HandKeyRotations (Utilities|Struct|BreakXRMotionControllerData _motioncontrollerdata)) (Math|Conversions|ToInteger(Byte) _enumvalue))))))
                (Components|PoseableMesh|SetBoneTransformbyName _left_hand (Utilities|RemoveSpaces _enumvalue) _adjustdata "ComponentSpace")
                (Transformation|SetWorldLocation _left_hand "0, 0, 0" false false))
              (:Right
                (Components|PoseableMesh|SetBoneTransformbyName (Variables|Default|GetRight%20Hand) (Utilities|RemoveSpaces _enumvalue) (Math|Transform|MakeTransform (Utilities|Array|Get(acopy) (.HandKeyPositions (Utilities|Struct|BreakXRMotionControllerData _motioncontrollerdata)) (Math|Conversions|ToInteger(Byte) _enumvalue)) (Class|KismetMathLibrary|QuatRotator (Utilities|Array|Get(acopy) (.HandKeyRotations (Utilities|Struct|BreakXRMotionControllerData _motioncontrollerdata)) (Math|Conversions|ToInteger(Byte) _enumvalue)))) "WorldSpace")))))))))

(event EventBeginPlay
  ;[1 1 1] Begin Play
  (CallFunction|PrepareforAR))

(event EventTick
  (params (DeltaSeconds :type Float%20%28single-precision%29))
  ;[1 1 1] Event Tick
  (CallFunction|TrackHands))

(event EventEndPlay
  (params (EndPlayReason :type EEndPlayReason%20Enum :default "Destroyed"))
  ;[1 1 1] End Play
  (Class|ARBlueprintLibrary|StopARSession))

(fn ConstructionScript)

(fn ConvertTransform
  (params (TrackedData :type Transform))
  (bind _left_hand (Variables|Default|GetLeft%20Hand))
  (bind _returnvalue (Transformation|GetWorldTransform _left_hand))
  (bind _returnvalue_2 (Math|Transform|ComposeTransforms TrackedData _returnvalue))
  (return (Math|Transform|MakeTransform (.location _returnvalue_2) (.rotation _returnvalue_2) (* (.scale _returnvalue_2) "1.000000,-1.000000,1.000000"))))