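; Hair dryer actor that blows physics objects along its up vector.
; While its Box overlaps anything, Tick runs nested loops sized by RangeX, RangeY and trace spacing, repeating the same box trace between two planes without a per-iteration offset.
; Each hit on a simulating component adds force at the impact point, scaled from MaxForce by frame delta time.
; BeginPlay caches the BP_Menu actor as HUD, which is otherwise unused.
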(event EventBeginPlay
  (bind _outactors (Actor|GetAllActorsOfClass "/Game/Blueprints/BP_Menu.BP_Menu_C"))
  (Variables|Default|SetHUD (Utilities|Array|Get(acopy) _outactors)))

(event Collision|EventActorBeginOverlap
  (params (OtherActor :type Actor%20Object%20Reference)))

(event EventTick
  (params (DeltaSeconds :type Float%20%28single-precision%29))
  (bind _plane (Variables|Default|GetPlane))
  (if true
    (if (> (Utilities|Array|Length (Class|PrimitiveComponent|GetOverlappingComponents (Variables|Default|GetBox))) 0)
      (for _index (range 0 (Math|Float|Truncate (/ (Variables|Default|GetRange%20X) (Variables|Default|GetDistanceBetweenLineTrace))))
        (for _index_2 (range 0 (Math|Float|Truncate (/ (Variables|Default|GetRange%20Y) (Variables|Default|GetDistanceBetweenLineTrace))))
          (bind (_outhit _returnvalue) (Collision|BoxTraceByChannel (Transformation|GetSocketLocation _plane "None") (Transformation|GetSocketLocation (Variables|Default|GetPlane1) "None") "5.000000,5.000000,5.000000" (Transformation|GetSocketRotation _plane "None") "TraceTypeQuery1" true 0 "None"))
          (if _returnvalue
            (if (Physics|IsSimulatingPhysics (.HitComponent (Collision|BreakHitResult _outhit)) "None")
              (Class|PrimitiveComponent|AddForceatLocation (.HitComponent (Collision|BreakHitResult _outhit)) (* (Math|Float|Lerp 0.0 (Variables|Default|GetMaxForce) (Utilities|Time|GetWorldDeltaSeconds)) (Transformation|GetActorUpVector)) (.ImpactPoint (Collision|BreakHitResult _outhit)) "None"))))))))

(fn ConstructionScript)