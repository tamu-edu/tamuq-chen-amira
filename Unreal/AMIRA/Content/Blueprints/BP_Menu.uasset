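; BP_Menu is a palm-up AR hand menu built with UX Tools for managing spatial mapping, object spawning and anchors.
; BeginPlay caches the ARPawn, Hair_Dryer and Pingpong, then binds buttons that toggle tabs, call pawn functions or cycle loaded anchors.
; Both spawn handlers bind to the SpawnPingpong button.
; Saving anchors pins both objects to local storage, while Tick polls the hairdryer toggle and saves object state on Exit press.
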(event OnConstraintActivated(UxtPalmUpConstraint)
  (Class|UxtUIElementComponent|SetUIVisibility (Variables|Default|GetUxtUIElement) "Show"))

(event OnConstraintDeactivated(UxtPalmUpConstraint)
  (Class|UxtUIElementComponent|SetUIVisibility (Variables|Default|GetUxtUIElement) "Hide"))

(event Custom|Initilize_anchor_tab
  (Utilities|FlowControl|Sequence
    (:then_0
      (Rendering|SetVisibility (Variables|Default|GetAnchor_tab) false true)
      (Rendering|SetVisibility (Variables|Default|GetMesh%20Tab) false true))
    (:then_1
      (bind _asuxt_pressable_button_actor (Utilities|Casting|CastToUxtPressableButtonActor (Variables|/Script/Engine.ChildActorComponent|GetChildActor (Variables|Default|GetAnchoring))))
      (EventDispatchers|BindEventtoOnButtonPressed (Variables|/Script/UXTools.UxtBasePressableButtonActor|GetButtonComponent _asuxt_pressable_button_actor) (delegate Custom|Tab%20Button%20Pressed)))
    (:then_2
      (bind _asuxt_pressable_switch_button_actor (Utilities|Casting|CastToUxtPressableSwitchButtonActor (Variables|/Script/Engine.ChildActorComponent|GetChildActor (Variables|Default|GetSpatial%20Mapping))))
      (EventDispatchers|BindEventtoOnToggled (Variables|/Script/UXTools.UxtPressableToggleButtonActor|GetToggleStateComponent _asuxt_pressable_switch_button_actor) (delegate Custom|Spatial_mapping))
      (bind _asuxt_pressable_switch_button_actor_2 (Utilities|Casting|CastToUxtPressableSwitchButtonActor (Variables|/Script/Engine.ChildActorComponent|GetChildActor (Variables|Default|GetShow%20Mesh))))
      (EventDispatchers|BindEventtoOnToggled (Variables|/Script/UXTools.UxtPressableToggleButtonActor|GetToggleStateComponent _asuxt_pressable_switch_button_actor_2) (delegate Custom|Show%20Spatial%20Mapped%20Mesh)))
    (:then_3
      (bind _asuxt_pressable_button_actor_2 (Utilities|Casting|CastToUxtPressableButtonActor (Variables|/Script/Engine.ChildActorComponent|GetChildActor (Variables|Default|GetSpawn%20Mesh))))
      (EventDispatchers|BindEventtoOnButtonPressed (Variables|/Script/UXTools.UxtBasePressableButtonActor|GetButtonComponent _asuxt_pressable_button_actor_2) (delegate Custom|Toggle_MeshSpawnTab))
      (bind _asuxt_pressable_button_actor_3 (Utilities|Casting|CastToUxtPressableButtonActor (Variables|/Script/Engine.ChildActorComponent|GetChildActor (Variables|Default|GetSpawn_Pingpong))))
      (EventDispatchers|BindEventtoOnButtonPressed (Variables|/Script/UXTools.UxtBasePressableButtonActor|GetButtonComponent _asuxt_pressable_button_actor_3) (delegate Custom|SpawnPingPong%20and%20Anchor))
      (bind _asuxt_pressable_button_actor_4 (Utilities|Casting|CastToUxtPressableButtonActor (Variables|/Script/Engine.ChildActorComponent|GetChildActor (Variables|Default|GetSpawn_Pingpong))))
      (EventDispatchers|BindEventtoOnButtonPressed (Variables|/Script/UXTools.UxtBasePressableButtonActor|GetButtonComponent _asuxt_pressable_button_actor_4) (delegate Custom|Spawn%20Hair%20Dryer)))
    (:then_4
      (bind _asuxt_pressable_button_actor_5 (Utilities|Casting|CastToUxtPressableButtonActor (Variables|/Script/Engine.ChildActorComponent|GetChildActor (Variables|Default|GetDeleteAnchor))))
      (EventDispatchers|BindEventtoOnButtonPressed (Variables|/Script/UXTools.UxtBasePressableButtonActor|GetButtonComponent _asuxt_pressable_button_actor_5) (delegate Custom|Delete%20Current%20Anchor))
      (bind _asuxt_pressable_button_actor_6 (Utilities|Casting|CastToUxtPressableButtonActor (Variables|/Script/Engine.ChildActorComponent|GetChildActor (Variables|Default|GetNextAnchor))))
      (EventDispatchers|BindEventtoOnButtonPressed (Variables|/Script/UXTools.UxtBasePressableButtonActor|GetButtonComponent _asuxt_pressable_button_actor_6) (delegate Custom|Show%20Next%20Anchor))
      (CallFunction|CycleAnchor)
      (bind _asuxt_pressable_button_actor_7 (Utilities|Casting|CastToUxtPressableButtonActor (Variables|/Script/Engine.ChildActorComponent|GetChildActor (Variables|Default|GetSave%20All%20Anchors))))
      (EventDispatchers|BindEventtoOnButtonPressed (Variables|/Script/UXTools.UxtBasePressableButtonActor|GetButtonComponent _asuxt_pressable_button_actor_7) (delegate Custom|Save%20All%20Actor%20Anchors)))))

(event Custom|SpawnPingPong%20and%20Anchor
  (params (Button :type Uxt%20Pressable%20Button%20Component%20Object%20Reference) (Pointer :type Uxt%20Pointer%20Component%20Object%20Reference))
  (Default|SpawnPingPongMesh (Variables|Default|GetAs%20ARPawn) (Variables|Default|GetAnchor%20Name)))

(event Custom|Save%20All%20Actor%20Anchors
  (params (Button :type Uxt%20Pressable%20Button%20Component%20Object%20Reference) (Pointer :type Uxt%20Pointer%20Component%20Object%20Reference))
  (bind _as_arpawn (Variables|Default|GetAs%20ARPawn))
  (bind _hair_dryer (Variables|Default|Gethair_dryer))
  (bind _pingpong (Variables|Default|GetPingpong))
  (bind _anchor (Variables|/Game/Blueprints/Hair_Dryer.Hair_Dryer_C|GetAnchor _hair_dryer))
  (bind _anchor_2 (Variables|/Game/Blueprints/pingpong.pingpong_C|GetAnchor _pingpong))
  (bind _anchorname (Variables|/Game/Blueprints/pingpong.pingpong_C|GetAnchorName _pingpong))
  (bind _anchorname_2 (Variables|/Game/Blueprints/Hair_Dryer.Hair_Dryer_C|GetAnchorName _hair_dryer))
  (bind _returnvalue (Utilities|String|StringToName _anchorname))
  (bind _returnvalue_2 (Utilities|String|StringToName _anchorname_2))
  (Utilities|FlowControl|Sequence
    (:then_0
      (bind _returnvalue_3 (Class|ARBlueprintLibrary|PinComponent _anchor (Transformation|GetWorldTransform _anchor) 0 _returnvalue_2))
      (Utilities|FlowControl|Delay 0.5)
      (Class|ARBlueprintLibrary|SaveARPintoLocalStore _returnvalue_2 _returnvalue_3)
      (Default|SaveLocalAnchor _as_arpawn _returnvalue_3 _returnvalue_2))
    (:then_1
      (bind _returnvalue_4 (Class|ARBlueprintLibrary|PinComponent _anchor_2 (Transformation|GetWorldTransform _anchor_2) 0))
      (Utilities|FlowControl|Delay 0.5)
      (Class|ARBlueprintLibrary|SaveARPintoLocalStore _returnvalue _returnvalue_4)
      (Default|SaveLocalAnchor _as_arpawn _returnvalue_4 _returnvalue))))

(event Custom|Show%20Spatial%20Mapped%20Mesh
  (params (ToggleState :type Uxt%20Toggle%20State%20Component%20Object%20Reference))
  (Default|SpatialMappingSetVisibility (Variables|Default|GetAs%20ARPawn) (Variables|/Script/UXTools.UxtToggleStateComponent|GetbIsChecked ToggleState)))

(event Custom|Tab%20Button%20Pressed
  (params (Button :type Uxt%20Pressable%20Button%20Component%20Object%20Reference) (Pointer :type Uxt%20Pointer%20Component%20Object%20Reference))
  (bind _anchor_tab (Variables|Default|GetAnchor_tab))
  (Utilities|FlowControl|FlipFlop
    (:A
      (Rendering|SetVisibility _anchor_tab true true))
    (:B
      (Rendering|SetVisibility _anchor_tab false true))))

(event Custom|Spatial_mapping
  (params (ToggleState :type Uxt%20Toggle%20State%20Component%20Object%20Reference))
  (Default|ToggleARSession (Variables|Default|GetAs%20ARPawn) (Variables|/Script/UXTools.UxtToggleStateComponent|GetbIsChecked ToggleState)))

(event Custom|Show%20Next%20Anchor
  (params (Button :type Uxt%20Pressable%20Button%20Component%20Object%20Reference) (Pointer :type Uxt%20Pointer%20Component%20Object%20Reference))
  (CallFunction|CycleAnchor))

(event Custom|Toggle_MeshSpawnTab
  (params (Button :type Uxt%20Pressable%20Button%20Component%20Object%20Reference) (Pointer :type Uxt%20Pointer%20Component%20Object%20Reference))
  (bind _mesh_tab (Variables|Default|GetMesh%20Tab))
  (Utilities|FlowControl|FlipFlop
    (:A
      (Rendering|SetVisibility _mesh_tab true true))
    (:B
      (Rendering|SetVisibility _mesh_tab false true))))

(event Custom|CycleAnchor
  (bind _returnvalue (Game|Player|GetPlayerPawn 0))
  (bind _asarpawn (Utilities|Casting|CastToARPawn _returnvalue))
  (bind _loadedarpins (Variables|/Game/Blueprints/ARPawn.ARPawn_C|GetLoadedARPins _asarpawn))
  (bind _returnvalue_2 (Utilities|Map|Length _loadedarpins))
  ;[1 1 1] Cycle Through Anchors
  (if (<= _returnvalue_2 0)
    (Rendering|Components|TextRender|SetText (Variables|Default|GetUxtTextRender_CurrentAnchor) (Utilities|Text|ToText(String) "No Anchors Loaded"))
    (else
      (if (>= (Variables|Default|GetCurrentLocalAnchor) (- _returnvalue_2 1))
        (Variables|Default|SetCurrentLocalAnchor 0)
        (else
          (Math|Integer|IncrementInt (Variables|Default|GetCurrentLocalAnchor)
            (:%20%20
              _))))
      (bind _keys (Utilities|Map|Keys _loadedarpins))
      (Rendering|Components|TextRender|SetText (Variables|Default|GetUxtTextRender_CurrentAnchor) (Utilities|Text|ToText(Name) (Utilities|Array|Get(acopy) _keys (Variables|Default|GetCurrentLocalAnchor)))))))

(event Custom|Spawn%20Hair%20Dryer
  (params (Button :type Uxt%20Pressable%20Button%20Component%20Object%20Reference) (Pointer :type Uxt%20Pointer%20Component%20Object%20Reference))
  (Default|SpawnHairDryer (Variables|Default|GetAs%20ARPawn) (Variables|Default|GetAnchor%20Name)))

(event Custom|Delete%20Current%20Anchor
  (params (Button :type Uxt%20Pressable%20Button%20Component%20Object%20Reference) (Pointer :type Uxt%20Pointer%20Component%20Object%20Reference))
  (Default|DeleteAnchor (.AsARPawn (Utilities|Casting|CastToARPawn (Game|Player|GetPlayerPawn 0))) (Utilities|String|StringToName (Utilities|String|ToString(Text) (Variables|/Script/Engine.TextRenderComponent|GetText (Variables|Default|GetUxtTextRender_CurrentAnchor))))))

(event EventTick
  (params (DeltaSeconds :type Float%20%28single-precision%29))
  (Utilities|FlowControl|Sequence
    (:then_0
      (Variables|Default|SetOn (Variables|/Script/UXTools.UxtToggleStateComponent|GetbIsChecked (Variables|/Script/UXTools.UxtPressableToggleButtonActor|GetToggleStateComponent (Variables|Default|GetHairblower_toggle)))))
    (:then_1
      (if (Utilities|Enum|Equal(Enum) (Class|UxtPressableButtonComponent|GetState (Variables|/Script/UXTools.UxtBasePressableButtonActor|GetButtonComponent (Variables|Default|GetExitButton))) "Pressed")
        (CallFunction|SaveGame)))))

(event EventBeginPlay
  (bind _asarpawn (Utilities|Casting|CastToARPawn (Game|Player|GetPlayerPawn 0)))
  (Variables|Default|SetAs%20ARPawn _asarpawn)
  (bind _returnvalue (Actor|GetActorOfClass "/Game/Blueprints/Hair_Dryer.Hair_Dryer_C"))
  (Variables|Default|Sethair_dryer _returnvalue)
  (bind _returnvalue_2 (Actor|GetActorOfClass "/Game/Blueprints/pingpong.pingpong_C"))
  (Variables|Default|SetPingpong _returnvalue_2)
  (bind _asuxt_pressable_toggle_button_actor (Utilities|Casting|CastToUxtPressableToggleButtonActor (Variables|/Script/Engine.ChildActorComponent|GetChildActor (Variables|Default|GetToggle_Hairdryer))))
  (Variables|Default|SetHairblower_toggle _asuxt_pressable_toggle_button_actor)
  (bind _asuxt_pressable_button_actor (Utilities|Casting|CastToUxtPressableButtonActor (Variables|/Script/Engine.ChildActorComponent|GetChildActor (Variables|Default|Getexit))))
  (Variables|Default|SetExitButton _asuxt_pressable_button_actor)
  (CallFunction|InitilizeAnchorTab))

(fn ConstructionScript)

(fn SaveGame
  (bind _returnvalue (SaveGame|DoesSaveGameExist "amira_1"))
  (if _returnvalue
    (Default|SaveGame (Variables|Default|GetPingpong))
    (Default|SaveGame (Variables|Default|Gethair_dryer))))