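; Ping-pong actor for an AR scene that persists its placement in a BP_Save slot.
; On BeginPlay, LoadGame restores the saved transform, or creates the save from the current one without caching it in AsBPSave.
; SaveGame writes the transform to the cached save but is not called here.
; UXT tap-to-place and ARPawn local-anchor code are disconnected, and SaveAnchorTransform is an empty event.
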(event Custom|AddInteraction)

(event Custom|End%20User%20Placement
  (params (TapToPlace :type Uxt%20Tap%20to%20Place%20Component%20Object%20Reference))
  (CallFunction|SaveAnchorTransform))

(event Custom|SaveAnchorTransform)

(event EventBeginPlay
  (CallFunction|LoadGame))

(fn ConstructionScript)

(fn LoadGame
  (bind _returnvalue (SaveGame|DoesSaveGameExist "amira_1"))
  (if _returnvalue
    (bind _returnvalue_2 (SaveGame|LoadGamefromSlot "amira_1"))
    (bind _asbp_save (Utilities|Casting|CastToBP_Save _returnvalue_2))
    (Variables|Default|SetAs%20BP%20Save _asbp_save)
    (Transformation|SetActorTransform (Variables|/Game/Blueprints/BP_Save.BP_Save_C|Getpingpong_pos _asbp_save))
    (else
      (bind _returnvalue_3 (SaveGame|CreateSaveGameObject "/Game/Blueprints/BP_Save.BP_Save_C"))
      (Variables|/Game/Blueprints/BP_Save.BP_Save_C|Setpingpong_pos _returnvalue_3 (Transformation|GetActorTransform))
      (SaveGame|SaveGametoSlot _returnvalue_3 "amira_1"))))

(fn SaveGame
  (bind _as_bp_save (Variables|Default|GetAs%20BP%20Save))
  (Variables|/Game/Blueprints/BP_Save.BP_Save_C|Setpingpong_pos _as_bp_save (Transformation|GetActorTransform))
  (SaveGame|SaveGametoSlot _as_bp_save "amira_1"))