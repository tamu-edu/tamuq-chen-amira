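; AR pawn for a head-mounted display that runs the AR session and spawns left and right UXT hand interaction actors.
; When RenderHands is on, Tick shows the hand meshes and runs hand tracking, which drives bones from tracked keypoints, with a Y-flipped scale for the left.
; Added world-classified AR geometry gets a wireframe material.
; Head and eye gaze traces are never triggered, and spatial anchor events are stubs beside disconnected pin save/load logic.
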(event OnAddTrackedGeometry(ARTrackableNotify)
  (params (TrackedGeometry :type AR%20Tracked%20Geometry%20Object%20Reference))
  (bind _returnvalue (Class|ARTrackedGeometry|GetUnderlyingMesh TrackedGeometry))
  ;[1 1 1] check
  (if (and (Utilities|Enum|Equal(Enum) (Class|ARTrackedGeometry|GetObjectClassification TrackedGeometry) "World") (Utilities|IsValid _returnvalue))
    (Class|MRMeshComponent|SetWireframeMaterial _returnvalue "/Engine/EngineDebugMaterials/WireframeMaterial.WireframeMaterial")))

(event Custom|EyeGraze_Tracking
  (bind _hmddata_location (Variables|Default|GetHMDData%20Location))
  (if (Class|EyeTrackerFunctionLibrary|IsEyeTrackerConnected)
    (bind (_outgazedata _returnvalue) (Class|EyeTrackerFunctionLibrary|GetGazeData))
    (if _returnvalue
      (Collision|LineTraceByChannel _hmddata_location (+ _hmddata_location (* (.gazedirection _outgazedata) 5e+02)) "TraceTypeQuery1" false 0 "ForOneFrame"))))

(event Custom|HeadOrientationTracking
  (bind _hmddata (Class|HeadMountedDisplayFunctionLibrary|GetHMDData self))
  (if (.bvalid _hmddata)
    (bind _output_get (Variables|Default|SetHMDData%20Location (.position _hmddata)))
    (Collision|LineTraceByChannel _output_get (+ _output_get (* (Math|Vector|GetForwardVector (Class|KismetMathLibrary|QuatRotator (.rotation _hmddata))) 5e+02)) "TraceTypeQuery1" false 0 "ForOneFrame" true "(R=0.129975,G=0.223225,B=1.000000,A=1.000000)")))

(event Custom|Hand_Tracking
  (bind _lefthand (Variables|Default|GetLeftHand))
  (for _index (range 0 1)
    (bind _motioncontrollerdata (Class|HeadMountedDisplayFunctionLibrary|GetMotionControllerData 0 (Utilities|Select :Index _index :Option%200 "Left" :Option%201 "Right")))
    (if (and (.bValid (Utilities|Struct|BreakXRMotionControllerData _motioncontrollerdata)) (Utilities|Enum|Equal(Enum) (.DeviceVisualType (Utilities|Struct|BreakXRMotionControllerData _motioncontrollerdata)) "Hand"))
      (bind _enumvalue (|ForEachEHandKeypoint)
        (:LoopBody
          (if (Transformation|DoesSocketExist (Variables|Default|GetRightHand) (Utilities|RemoveSpaces _enumvalue))
            (switch Utilities|FlowControl|Switch|SwitchonEControllerHand (.HandIndex (Utilities|Struct|BreakXRMotionControllerData _motioncontrollerdata))
              (:Left
                (bind _adjustedtransform (CallFunction|ConvertTransform (Math|Transform|MakeTransform (Utilities|Array|Get(acopy) (.HandKeyPositions (Utilities|Struct|BreakXRMotionControllerData _motioncontrollerdata)) (Math|Conversions|ToInteger(Byte) _enumvalue)) (Class|KismetMathLibrary|QuatRotator (Utilities|Array|Get(acopy) (.HandKeyRotations (Utilities|Struct|BreakXRMotionControllerData _motioncontrollerdata)) (Math|Conversions|ToInteger(Byte) _enumvalue))))))
                (Components|PoseableMesh|SetBoneTransformbyName _lefthand (Utilities|RemoveSpaces _enumvalue) _adjustedtransform "ComponentSpace")
                (Transformation|SetWorldLocation _lefthand "0, 0, 0" false false))
              (:Right
                (Components|PoseableMesh|SetBoneTransformbyName (Variables|Default|GetRightHand) (Utilities|RemoveSpaces _enumvalue) (Math|Transform|MakeTransform (Utilities|Array|Get(acopy) (.HandKeyPositions (Utilities|Struct|BreakXRMotionControllerData _motioncontrollerdata)) (Math|Conversions|ToInteger(Byte) _enumvalue)) (Class|KismetMathLibrary|QuatRotator (Utilities|Array|Get(acopy) (.HandKeyRotations (Utilities|Struct|BreakXRMotionControllerData _motioncontrollerdata)) (Math|Conversions|ToInteger(Byte) _enumvalue)))) "WorldSpace")))))))))

(event Custom|Initalize%20SpatialAnchor)

(event Custom|SpawnHandInteraction
  (bind _returnvalue (Math|Transform|MakeTransform "0, 0, 0"))
  (bind _self self)
  (Game|SpawnActorfromClass "/Script/UXTools.UxtHandInteractionActor" _returnvalue "Undefined" _self false "Left" 0)
  (Game|SpawnActorfromClass "/Script/UXTools.UxtHandInteractionActor" _returnvalue "Undefined" _self false "Right" 0))

(event Custom|Save%20Spatial%20Anchor)

(event Custom|Load%20ARPin)

(event EventBeginPlay
  (if (Class|HeadMountedDisplayFunctionLibrary|IsHeadMountedDisplayEnabled)
    (Class|ARBlueprintLibrary|StartARSession "/Game/ARSessionConfig.ARSessionConfig")
    (Class|HeadMountedDisplayFunctionLibrary|SetTrackingOrigin "Floor")
    (CallFunction|SpawnHandInteraction)))

(event Collision|EventActorBeginOverlap
  (params (OtherActor :type Actor%20Object%20Reference)))

(event EventTick
  (params (DeltaSeconds :type Float%20%28single-precision%29))
  (bind _righthand (Variables|Default|GetRightHand))
  (bind _righthand_2 (Variables|Default|GetRightHand))
  (if (Variables|Default|GetRenderHands)
    (CallFunction|HandTracking)
    (if (not (Rendering|IsVisible _righthand))
      (Rendering|SetVisibility _righthand true false))
    (elif (not (Rendering|IsVisible _righthand_2))
      (Rendering|SetVisibility _righthand_2 false false))))

(event EventEndPlay
  (params (EndPlayReason :type EEndPlayReason%20Enum :default "Destroyed"))
  (Class|ARBlueprintLibrary|StopARSession))

(fn ConstructionScript)

(fn ConvertTransform
  (params (TrackedData :type Transform))
  (bind _lefthand (Variables|Default|GetLeftHand))
  (bind _returnvalue (Transformation|GetWorldTransform _lefthand))
  (bind _returnvalue_2 (Math|Transform|ComposeTransforms TrackedData _returnvalue))
  (return (Math|Transform|MakeTransform (.location _returnvalue_2) (.rotation _returnvalue_2) (* (.scale _returnvalue_2) "1.000000,-1.000000,1.000000"))))