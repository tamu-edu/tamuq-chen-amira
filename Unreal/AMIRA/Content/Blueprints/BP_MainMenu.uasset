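; BP_MainMenu is a main menu actor that uses a UXT pressable button to set the game-started flag and toggle the hair dryer.
; BeginPlay caches the first Hair_Dryer actor in the level.
; Tick polls the button in the On child actor, setting IsGameStarted and unhiding the dryer's root component only while it reads Pressed.
; The hidden-in-game change does not propagate to child components.
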(event EventBeginPlay
  (bind _outactors (Actor|GetAllActorsOfClass "/Game/Blueprints/Hair_Dryer.Hair_Dryer_C"))
  (Variables|Default|SetHair_Dryer (Utilities|Array|Get(acopy) _outactors)))

(event Collision|EventActorBeginOverlap
  (params (OtherActor :type Actor%20Object%20Reference)))

(event EventTick
  (params (DeltaSeconds :type Float%20%28single-precision%29))
  (bind _hair_dryer (Variables|Default|GetHair_Dryer))
  (bind _defaultsceneroot (Variables|/Game/Blueprints/Hair_Dryer.Hair_Dryer_C|GetDefaultSceneRoot _hair_dryer))
  (bind _asuxt_pressable_button_actor (Utilities|Casting|CastToUxtPressableButtonActor (Variables|/Script/Engine.ChildActorComponent|GetChildActor (Variables|Default|GetOn))))
  (if (Utilities|Enum|Equal(Enum) (Class|UxtPressableButtonComponent|GetState (Variables|/Script/UXTools.UxtBasePressableButtonActor|GetButtonComponent _asuxt_pressable_button_actor)) "Pressed")
    (Variables|Default|SetIsGameStarted? true)
    (Development|SetHiddeninGame _defaultsceneroot false false)
    (else
      (Variables|Default|SetIsGameStarted? false)
      (Development|SetHiddeninGame _defaultsceneroot true false))))

(fn ConstructionScript)