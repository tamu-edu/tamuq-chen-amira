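; AR headset pawn that runs the AR session and manages anchored ping-pong and hair dryer props.
; Drives hand mesh bones from tracked keypoints, mirroring the left, alongside spawned MRTK UXT hand interaction actors.
; Provides head and eye gaze traces, plus spatial mapping meshes with toggleable wireframe.
; Spawns props head-aligned, and reloads local-store AR pins to respawn and attach them by name, refreshing BP_Menu when anchors change.
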(event OnUpdateTrackedGeometry(ARTrackableNotify)
  (params (TrackedGeometry :type AR%20Tracked%20Geometry%20Object%20Reference))
  (bind _returnvalue (Class|ARTrackedGeometry|GetUnderlyingMesh TrackedGeometry))
  ;[1 1 1] Spatial Mapping
  (Utilities|IsValid _returnvalue
    (:Is%20Valid
      (if (Utilities|Enum|Equal(Enum) (.status (Class|ARBlueprintLibrary|GetARSessionStatus)) "Running")
        (Utilities|Array|AddUnique (Variables|Default|GetTrackedGeometry) _returnvalue)
        (if (Variables|Default|GetspatialMappingRenderMesh)
          (CallFunction|SpatialMappingSetVisibility true))))))

(event Custom|EyeGraze_Tracking
  (bind _hmddata_location (Variables|Default|GetHMDData%20Location))
  ;[1 1 1] Eye Graze Tracking
  (if (Class|EyeTrackerFunctionLibrary|IsEyeTrackerConnected)
    (bind (_outgazedata _returnvalue) (Class|EyeTrackerFunctionLibrary|GetGazeData))
    (if _returnvalue
      (Collision|LineTraceByChannel _hmddata_location (+ _hmddata_location (* (.gazedirection _outgazedata) 5e+02)) "TraceTypeQuery1" false 0 "ForOneFrame"))))

(event Custom|HeadOrientationTracking
  ;[1 1 1] Head Orientation Tracking
  (bind _hmddata (Class|HeadMountedDisplayFunctionLibrary|GetHMDData self))
  (if (.bvalid _hmddata)
    (bind _output_get (Variables|Default|SetHMDData%20Location (.position _hmddata)))
    (bind _outhit (Collision|LineTraceByChannel _output_get (+ _output_get (* (Math|Vector|GetForwardVector (Class|KismetMathLibrary|QuatRotator (.rotation _hmddata))) 5e+02)) "TraceTypeQuery1" false 0 "ForOneFrame" true "(R=0.129975,G=0.223225,B=1.000000,A=1.000000)"))
    (Variables|Default|SetHead%20Tracking%20Hit _outhit)))

(event Custom|AttachActortoPin
  (params (ComponentToPin :type Scene%20Component%20Object%20Reference) (DebugName :type Name))
  ;[1 1 1] Setting loaded actor to saved pin
  (bind _values (Utilities|Map|Values (Variables|Default|GetLoadedARPins)))
  (for _array_element _values
    (if (== (Class|ARPin|GetDebugName _array_element) DebugName)
      (Utilities|IsValid (Class|ARPin|GetPinnedComponent _array_element)
        (:Is%20Valid
          (Transformation|AttachComponentToComponent (Components|GetOwner ComponentToPin) (Class|ARPin|GetPinnedComponent _array_element) "None" "SnapToTarget" "SnapToTarget" "KeepRelative" true))
        (:Is%20Not%20Valid
          (Class|ARBlueprintLibrary|PinComponenttoARPin ComponentToPin _array_element))))))

(event Custom|DeleteAnchor
  (params (AnchorName :type Name) (RemoveBPAnchor :type Actor%20Object%20Reference))
  ;[1 1 1] Delete Current Anchor
  (Class|ARBlueprintLibrary|RemoveARPinfromLocalStore AnchorName)
  (Utilities|Map|Remove (Variables|Default|GetLoadedARPins) AnchorName)
  (Default|CycleAnchor (Variables|Default|GetBP_Menu)))

(event Custom|Load%20Local%20Anchors
  (bind _pingpong (Variables|Default|GetPingpong))
  (bind _hairdryer (Variables|Default|GetHairDryer))
  ;[1 1 1] Load AR Pins
  (Utilities|FlowControl|Sequence
    (:then_0
      (Utilities|IsValid _pingpong
        (:Is%20Valid
          (Actor|DestroyActor _pingpong))
        (:Is%20Not%20Valid
          _))
      (Utilities|IsValid _hairdryer
        (:Is%20Valid
          (Actor|DestroyActor _hairdryer))))
    (:then_1
      (Utilities|Map|Clear (Variables|Default|GetLoadedARPins))
      (bind _returnvalue (Class|ARBlueprintLibrary|LoadARPinsfromLocalStore))
      (Variables|Default|SetLoadedARPins _returnvalue)
      (Default|CycleAnchor (Variables|Default|GetBP_Menu))
      (CallFunction|SpawnActorMesh))))

(event Custom|Spawn%20actor%20Mesh
  ;[1 1 1] Spawning Meshes after loading anchors
  (bind _values (Utilities|Map|Values (Variables|Default|GetLoadedARPins)))
  (for _array_element _values
    (if (== (Utilities|String|StringToName (Utilities|String|ToString(Name) (Class|ARPin|GetDebugName _array_element))) "pingpong")
      (bind _returnvalue (Game|SpawnActorfromClass "/Game/Blueprints/pingpong.pingpong_C" (Math|Transform|MakeTransform "0, 0, 0" "0, 0, 0" "1.000000,1.000000,1.000000") "AlwaysSpawn" 0 (Utilities|String|ToString(Name) (Class|ARPin|GetDebugName _array_element)) 0))
      (CallFunction|AttachActortoPin (Variables|/Game/Blueprints/pingpong.pingpong_C|GetAnchor _returnvalue) (Class|ARPin|GetDebugName _array_element))
      (elif (== (Utilities|String|StringToName (Utilities|String|ToString(Name) (Class|ARPin|GetDebugName _array_element))) "hairdryer")
        (bind _returnvalue_2 (Game|SpawnActorfromClass "/Game/Blueprints/Hair_Dryer.Hair_Dryer_C" (Math|Transform|MakeTransform "0, 0, 0" "0, 0, 0" "1.000000,1.000000,1.000000") "AlwaysSpawn" 0 "hairdryer" 0))
        (CallFunction|AttachActortoPin (Variables|/Game/Blueprints/Hair_Dryer.Hair_Dryer_C|GetAnchor _returnvalue_2) (Class|ARPin|GetDebugName _array_element))))))

(event Custom|Hand_Tracking
  (bind _lefthand (Variables|Default|GetLeftHand))
  ;[1 1 1] Hand Tracking
  (for _index (range 0 1)
    (bind _motioncontrollerdata (Class|HeadMountedDisplayFunctionLibrary|GetMotionControllerData 0 (Utilities|Select :Index _index :Option%200 "Left" :Option%201 "Right")))
    (if (and (.bValid (Utilities|Struct|BreakXRMotionControllerData _motioncontrollerdata)) (Utilities|Enum|Equal(Enum) (.DeviceVisualType (Utilities|Struct|BreakXRMotionControllerData _motioncontrollerdata)) "Hand"))
      (bind _enumvalue (|ForEachEHandKeypoint)
        (:LoopBody
          (if (Transformation|DoesSocketExist (Variables|Default|GetRightHand) (Utilities|RemoveSpaces _enumvalue))
            (switch Utilities|FlowControl|Switch|SwitchonEControllerHand (.HandIndex (Utilities|Struct|BreakXRMotionControllerData _motioncontrollerdata))
              (:Left
                (bind _adjustedtransform (CallFunction|ConvertTransform (Math|Transform|MakeTransform (Utilities|Array|Get(acopy) (.HandKeyPositions (Utilities|Struct|BreakXRMotionControllerData _motioncontrollerdata)) (Math|Conversions|ToInteger(Byte) _enumvalue)) (Class|KismetMathLibrary|QuatRotator (Utilities|Array|Get(acopy) (.HandKeyRotations (Utilities|Struct|BreakXRMotionControllerData _motioncontrollerdata)) (Math|Conversions|ToInteger(Byte) _enumvalue))))))
                (Components|PoseableMesh|SetBoneTransformbyName _lefthand (Utilities|RemoveSpaces _enumvalue) _adjustedtransform "ComponentSpace")
                (Transformation|SetWorldLocation _lefthand "0, 0, 0" false false))
              (:Right
                (Components|PoseableMesh|SetBoneTransformbyName (Variables|Default|GetRightHand) (Utilities|RemoveSpaces _enumvalue) (Math|Transform|MakeTransform (Utilities|Array|Get(acopy) (.HandKeyPositions (Utilities|Struct|BreakXRMotionControllerData _motioncontrollerdata)) (Math|Conversions|ToInteger(Byte) _enumvalue)) (Class|KismetMathLibrary|QuatRotator (Utilities|Array|Get(acopy) (.HandKeyRotations (Utilities|Struct|BreakXRMotionControllerData _motioncontrollerdata)) (Math|Conversions|ToInteger(Byte) _enumvalue)))) "WorldSpace")))))))))

(event Custom|SaveLocalAnchor
  (params (Component%20To%20Pin :type AR%20Pin%20Object%20Reference) (Debug%20Name :type Name))
  ;[1 1 1] Save Local Anchors
  (Utilities|Map|Add (Variables|Default|GetLoadedARPins) Debug%20Name Component%20To%20Pin))

(event Custom|SpawnHandInteraction
  (bind _returnvalue (Math|Transform|MakeTransform "0, 0, 0"))
  (bind _self self)
  ;[1 1 1] Overlay Hand with MRTK Hand mesh
  (Game|SpawnActorfromClass "/Script/UXTools.UxtHandInteractionActor" _returnvalue "Undefined" _self false "Left" 0)
  (Game|SpawnActorfromClass "/Script/UXTools.UxtHandInteractionActor" _returnvalue "Undefined" _self false "Right" 0))

(event Custom|Spawn_HairDryer
  (params (Actor%20Name :type String))
  ;[1 1 1] Spawn Hair Dryer
  (if (and (Class|ARBlueprintLibrary|IsARPinLocalStoreSupported) (Class|ARBlueprintLibrary|IsARPinLocalStoreReady))
    (Game|SpawnActorfromClass "/Game/Blueprints/Hair_Dryer.Hair_Dryer_C" (Math|Transform|MakeTransform (Utilities|AligntoHead) "0, 0, 0" "1.000000,1.000000,1.000000") "AlwaysSpawn" 0 Actor%20Name 0)
    (else
      (Development|PrintString "[BP_Pawn | AddLocalAnchor] + + + ARPin Local Store is NOT ready + + +") ; Warn User that the Local Store is not ready
    )))

(event Custom|DeleteAllAnchors
  (bind _bp_menu (Variables|Default|GetBP_Menu))
  ;[1 1 1] Delete All AR Anchors
  (Class|ARBlueprintLibrary|RemoveAllARPinsfromLocalStore)
  (Utilities|Map|Clear (Variables|Default|GetLoadedARPins))
  (Utilities|IsValid _bp_menu
    (:Is%20Valid
      (Default|CycleAnchor _bp_menu))))

(event Custom|SpatialMapping_SetVisibility
  (params (Visible :type Boolean))
  (bind _trackedgeometry (Variables|Default|GetTrackedGeometry))
  ;[1 1 1] Spatial Mapping
  (Variables|Default|SetspatialMappingRenderMesh Visible)
  (for _array_element _trackedgeometry
    (Utilities|IsValid _array_element
      (:Is%20Valid
        (Rendering|Material|SetMaterial _array_element 0 (select (Variables|Default|GetspatialMappingRenderMesh) "/Engine/EngineDebugMaterials/WireframeMaterial.WireframeMaterial" 0)))
      (:Is%20Not%20Valid
        (Utilities|Array|RemoveItem _trackedgeometry _array_element)))))

(event Custom|ToggleARSession
  (params (Active :type Boolean))
  ;[1 1 1] Spatial Mapping
  (if Active
    (Class|ARBlueprintLibrary|StartARSession "/Game/ARSessionConfig.ARSessionConfig")
    (else
      (Class|ARBlueprintLibrary|PauseARSession))))

(event Custom|SpawnPingPongMesh
  (params (Anchor%20Name :type String))
  ;[1 1 1] Spawn PingPong
  (if (and (Class|ARBlueprintLibrary|IsARPinLocalStoreSupported) (Class|ARBlueprintLibrary|IsARPinLocalStoreReady))
    (Game|SpawnActorfromClass "/Game/Blueprints/pingpong.pingpong_C" (Math|Transform|MakeTransform (Utilities|AligntoHead) "0, 0, 0" "1.000000,1.000000,1.000000") "AlwaysSpawn" 0 Anchor%20Name 0)
    (else
      (Development|PrintString "[BP_Pawn | AddLocalAnchor] + + + ARPin Local Store is NOT ready + + +") ; Warn User that the Local Store is not ready
    )))

(event EventBeginPlay
  ;[1 1 1] BeginPlay - Initialize Variables and AR Session
  (if (Class|HeadMountedDisplayFunctionLibrary|IsHeadMountedDisplayEnabled)
    (Class|ARBlueprintLibrary|StartARSession "/Game/ARSessionConfig.ARSessionConfig")
    (Class|HeadMountedDisplayFunctionLibrary|SetTrackingOrigin "Floor")
    (CallFunction|SpawnHandInteraction)
    (bind _returnvalue (Actor|GetActorOfClass "/Game/Blueprints/BP_Menu.BP_Menu_C"))
    (Variables|Default|SetBP_Menu _returnvalue)
    (bind _returnvalue_2 (Actor|GetActorOfClass "/Game/Blueprints/pingpong.pingpong_C"))
    (Variables|Default|SetPingpong _returnvalue_2)
    (bind _returnvalue_3 (Actor|GetActorOfClass "/Game/Blueprints/Hair_Dryer.Hair_Dryer_C"))
    (Variables|Default|SetHairDryer _returnvalue_3)))

(event EventTick
  (params (DeltaSeconds :type Float%20%28single-precision%29))
  (bind _righthand (Variables|Default|GetRightHand))
  (bind _righthand_2 (Variables|Default|GetRightHand))
  ;[1 1 1] Event Tick for Hand Tracking
  (if (Variables|Default|GetRenderHands)
    (CallFunction|HandTracking)
    (if (not (Rendering|IsVisible _righthand))
      (Rendering|SetVisibility _righthand true false))
    (elif (not (Rendering|IsVisible _righthand_2))
      (Rendering|SetVisibility _righthand_2 false false))))

(event EventEndPlay
  (params (EndPlayReason :type EEndPlayReason%20Enum :default "Destroyed"))
  ;[1 1 1] EndPlay
  (Class|ARBlueprintLibrary|StopARSession))

(fn ConstructionScript)

(fn ConvertTransform
  (params (TrackedData :type Transform))
  (bind _lefthand (Variables|Default|GetLeftHand))
  (bind _returnvalue (Transformation|GetWorldTransform _lefthand))
  (bind _returnvalue_2 (Math|Transform|ComposeTransforms TrackedData _returnvalue))
  (return (Math|Transform|MakeTransform (.location _returnvalue_2) (.rotation _returnvalue_2) (* (.scale _returnvalue_2) "1.000000,-1.000000,1.000000"))))